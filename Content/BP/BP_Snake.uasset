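; Player-controlled snake for a Snake game, steered with WASD along the X and Y axes without direct reversals.
; Every Tick sweeps the head one mesh-width along Direction and shifts each Tail actor into the previous segment's location.
; AddTail spawns and stores a scaled-down segment behind the head; the loop that adds starting segments is disconnected.
; Overlapping a Tail destroys all segments, calls LoseGame through an interface and destroys the snake.
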(event `self.ReceiveActorBeginOverlap`
  (params (OtherActor :type "Actor Object Reference"))
  (cast `/Game/BP/Tail` OtherActor)
  (`self.StopGame`)
  (`/Game/UBP_Interface.LoseGame` (`self.Interface`))
  (`self.K2_DestroyActor`))

(event `self.ReceiveTick`
  (params (DeltaSeconds :type "Float (single-precision)"))
  (set `self.PrevLocation` (`SceneComponent.K2_GetComponentLocation` (`self.Head`)))
  (`SceneComponent.K2_AddWorldOffset` (`self.Head`) (* (`self.StepSize`) (`self.Direction`)) true false)
  (for _array_element (`self.SnakeMesh`)
    (bind _defaultsceneroot (`/Game/BP/Tail.DefaultSceneRoot` _array_element))
    (set `self.TailCurrLocation` (`SceneComponent.K2_GetComponentLocation` _defaultsceneroot))
    (`SceneComponent.K2_SetWorldLocation` _defaultsceneroot (`self.PrevLocation`) true false)
    (set `self.PrevLocation` (`self.TailCurrLocation`))))

(event `self.ReceiveBeginPlay`
  (bind (_min _max) (`StaticMeshComponent.GetLocalBounds` (`self.Head`)))
  (set `self.StepSize` (- (.x _max) (.x _min))))

(event `Key|W`
  (params (Key :type "Key Structure"))
  (bind _direction_x (`KismetMathLibrary.BreakVector` (`self.Direction`)))
  (:`Pressed`
    (if (== _direction_x 0.0)
      (set `self.Direction` (1.0 0.0 0.0)))))

(event `Key|S`
  (params (Key :type "Key Structure"))
  (bind _direction_x (`KismetMathLibrary.BreakVector` (`self.Direction`)))
  (:`Pressed`
    (if (== _direction_x 0.0)
      (set `self.Direction` (-1.0 0.0 0.0)))))

(event `Key|D`
  (params (Key :type "Key Structure"))
  (bind (_direction_x _direction_y) (`KismetMathLibrary.BreakVector` (`self.Direction`)))
  (:`Pressed`
    (if (== _direction_y 0.0)
      (set `self.Direction` (0.0 1.0 0.0)))))

(event `Key|A`
  (params (Key :type "Key Structure"))
  (bind (_direction_x _direction_y) (`KismetMathLibrary.BreakVector` (`self.Direction`)))
  (:`Pressed`
    (if (== _direction_y 0.0)
      (set `self.Direction` (0.0 -1.0 0.0)))))

(fn `AddTail`
  (bind _returnvalue (`|SpawnActorFromClass` "/Game/BP/Tail.Tail_C" (`KismetMathLibrary.MakeTransform` (- (`SceneComponent.K2_GetComponentLocation` (`self.Head`)) (* (`self.Direction`) (`self.StepSize`))) (struct) (0.6 0.6 0.6)) "Undefined" "OverrideRootScale" null null))
  (`KismetArrayLibrary.Array_Add` (`self.SnakeMesh`) _returnvalue))

(fn `StopGame`
  (for _array_element (`self.SnakeMesh`)
    (`self.K2_DestroyActor` _array_element))
  (`KismetArrayLibrary.Array_Clear` (`self.SnakeMesh`)))

(fn `UserConstructionScript`)