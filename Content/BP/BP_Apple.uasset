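; Apple pickup actor for a Snake game that the snake eats to grow and score.
; On BeginPlay it moves its cube to a random integer X/Y position within the min and max bounds at a fixed height.
; Overlap with a BP_Snake adds a tail segment, relocates the apple and adds a point through the interface reference.
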(event `OnAppleEat`
  (params (Snake :type "/Game/BP/BP_Snake Object Reference"))
  (`/Game/BP/BP_Snake.AddTail` Snake)
  (`self.MoveApple`)
  (`/Game/UBP_Interface.AddScore` (`self.Interface`) 1))

(event `self.ReceiveBeginPlay`
  (`self.MoveApple`))

(event `self.ReceiveActorBeginOverlap`
  (params (OtherActor :type "Actor Object Reference"))
  (bind _asbp_snake (cast `/Game/BP/BP_Snake` OtherActor))
  (`self.OnAppleEat` _asbp_snake))

(fn `MoveApple`
  (bind (_maxcoords_x _maxcoords_y) (`KismetMathLibrary.BreakVector` (`self.MaxCoords`)))
  (bind (_mincoords_x _mincoords_y) (`KismetMathLibrary.BreakVector` (`self.MinCoords`)))
  (bind _maxcoords_x_2 (`KismetMathLibrary.BreakVector` (`self.MaxCoords`)))
  (bind _mincoords_x_2 (`KismetMathLibrary.BreakVector` (`self.MinCoords`)))
  (`SceneComponent.K2_SetWorldLocation` (`self.Cube`) (`KismetMathLibrary.MakeVector` (`KismetMathLibrary.Conv_IntToDouble` (`KismetMathLibrary.RandomIntegerInRange` (`KismetMathLibrary.FTrunc` _mincoords_x_2) (`KismetMathLibrary.FTrunc` _maxcoords_x_2))) (`KismetMathLibrary.Conv_IntToDouble` (`KismetMathLibrary.RandomIntegerInRange` (`KismetMathLibrary.FTrunc` _mincoords_y) (`KismetMathLibrary.FTrunc` _maxcoords_y))) 100.0) false false))

(fn `UserConstructionScript`)